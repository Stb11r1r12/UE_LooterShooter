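; BP_Character is a looter-shooter character Blueprint with basic keyboard movement.
; Pressing W, S, A or D teleports the actor a fixed step along the world X or Y axis via SetActorLocation, without sweep or collision checks.
; Movement happens once per key press, ignores facing direction and uses no movement component input.
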(event Input|KeyboardEvents|D
  (params (Key :type Key%20Structure :default "None"))
  (:Pressed
    (Transformation|SetActorLocation (+ (Transformation|GetActorLocation) "0.000000,100.000000,0.000000") false false)))

(event Input|KeyboardEvents|W
  (params (Key :type Key%20Structure :default "None"))
  (:Pressed
    (Transformation|SetActorLocation (+ (Transformation|GetActorLocation) "100.000000,0.000000,0.000000") false false)))

(event Input|KeyboardEvents|S
  (params (Key :type Key%20Structure :default "None"))
  (:Pressed
    (Transformation|SetActorLocation (+ (Transformation|GetActorLocation) "-100.000000,0.000000,0.000000") false false)))

(event Input|KeyboardEvents|A
  (params (Key :type Key%20Structure :default "None"))
  (:Pressed
    (Transformation|SetActorLocation (+ (Transformation|GetActorLocation) "0.000000,-100.000000,0.000000") false false)))

(fn ConstructionScript)