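; BP_MyActor is an actor Blueprint that initializes and prints basic combat and movement stats such as HP, damage and speed.
; On BeginPlay it fills current HP from max HP, derives outgoing damage through Buff and movement speed through MSBuff, printing debug values along the way.
; MSBuff overrides the parent function and halves its result.
; The PrintActorData event prints a summary of health, base damage, movement speed and interaction radius.
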(event EventPrintActorData
  (bind _hp (Variables|Default|GetHP))
  (bind _basedamage (Variables|Default|GetbaseDamage))
  (bind _movementspeed (Variables|Default|GetmovementSpeed))
  (bind _interactionradius (Variables|Default|GetinteractionRadius))
  (bind _returnvalue (Utilities|String|ToString(Float) (.maxhp _hp)))
  (bind _returnvalue_2 (Utilities|String|ToString(Float) (.currenthp _hp)))
  (bind _returnvalue_3 (Utilities|String|ToString(Integer) _basedamage))
  (bind _returnvalue_4 (Utilities|String|ToString(Float) _movementspeed))
  (bind _returnvalue_5 (Utilities|String|ToString(Float) _interactionradius))
  (bind _returnvalue_6 (Utilities|String|Append "MaxHP: " _returnvalue " CurrentHP: " _returnvalue_2 " Base Damage: " _returnvalue_3 " Movement Speed: " _returnvalue_4 " Interaction Radius:" _returnvalue_5))
  (Development|PrintString _returnvalue_6 true true "(R=0.000000,G=0.660000,B=1.000000,A=1.000000)" 2.0 (Utilities|String|StringToName _returnvalue_6)))

(event EventBeginPlay
  (bind _hp (Variables|Default|GetHP))
  (Development|PrintString (Utilities|String|Append "Max HP: " (Utilities|String|ToString(Float) (.maxhp _hp)) " Curr HP:" (Utilities|String|ToString(Float) (.currenthp _hp))))
  (Utilities|Struct|SetmembersinHPStruct (Variables|Default|GetHP) (.maxhp (Variables|Default|GetHP)))
  (bind _returnvalue (Class|MyActor|Buff (Variables|Default|GetBuf) (Variables|Default|GetDebuf)))
  (bind _output_get (Variables|Default|SetOutgoingDamage _returnvalue))
  (Development|PrintString (Utilities|String|Append "Outgoing Damage: " (Utilities|String|ToString(Float) _output_get)))
  (bind _returnvalue_2 (CallFunction|MSBuff (Variables|Default|GetMovementSpeedMultiplier)))
  (bind _output_get_2 (Variables|Default|SetmovementSpeed _returnvalue_2))
  (Development|PrintString (Utilities|String|ToString(Float) _output_get_2)))

(fn ConstructionScript)

(fn MSBuff
  (params (multiply :type Float%20%28single-precision%29))
  (bind _returnvalue (|CallParentFunction multiply))
  (return (/ _returnvalue 2.0)))