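; Elevator actor that moves its Plane component vertically as a platform, triggered by overlap events.
; Beginning an overlap on Box plays an upward timeline, and ending an overlap on Plane plays a second timeline with a downward offset.
; Both timelines feed MovingPlatform, which lerps from the actor's location, not the platform's current position.
; A shared IsWorking flag ignores new triggers until the running timeline finishes.
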(event OnComponentEndOverlap(Plane)
  (params (OverlappedComponent :type Primitive%20Component%20Object%20Reference) (OtherActor :type Actor%20Object%20Reference) (OtherComp :type Primitive%20Component%20Object%20Reference) (OtherBodyIndex :type Integer))
  (if (not (Variables|Default|GetisWorking))
    (Variables|Default|SetisWorking true)
    (bind _newtrack_1 (Timeline|Timeline_0 Play)
      (:Update
        (CallFunction|MovingPlatform _newtrack_1 (Variables|Default|GetPlane) "0.000000,0.000000,-1000.000000"))
      (:Finished
        (Variables|Default|SetisWorking false)))))

(event OnComponentBeginOverlap(Box)
  (params (OverlappedComponent :type Primitive%20Component%20Object%20Reference) (OtherActor :type Actor%20Object%20Reference) (OtherComp :type Primitive%20Component%20Object%20Reference) (OtherBodyIndex :type Integer) (bFromSweep :type Boolean) (SweepResult :type Hit%20Result%20Structure%20%28by%20ref%29))
  (if (not (Variables|Default|GetisWorking))
    (Variables|Default|SetisWorking true)
    (bind _newtrack_1 (Timeline|Timeline Play)
      (:Update
        (CallFunction|MovingPlatform _newtrack_1 (Variables|Default|GetPlane) "0.000000,0.000000,1000.000000"))
      (:Finished
        (Variables|Default|SetisWorking false)))))

(fn ConstructionScript)

(fn MovingPlatform
  (params (Alpha :type Float%20%28single-precision%29) (SceneComponent :type Scene%20Component%20Object%20Reference) (VectorToMove :type Vector))
  (bind _returnvalue (Transformation|GetActorLocation))
  (Transformation|SetWorldLocation SceneComponent (Math|Vector|Lerp(Vector) _returnvalue (+ _returnvalue VectorToMove) Alpha) false false))