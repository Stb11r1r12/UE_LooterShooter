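; BP_Svetofor is a traffic light actor that changes its state each time something overlaps its sphere.
; On BeginPlay it caches every row of the DT_Svetovor data table into an array.
; Each overlap uses GetDTElem to pick a row by overlap count modulo three, cycling the first three rows.
; That row sets the point light's color and intensity, then its name, description and the count are printed to screen.
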(event OnComponentBeginOverlap(Sphere)
  (params (OverlappedComponent :type Primitive%20Component%20Object%20Reference) (OtherActor :type Actor%20Object%20Reference) (OtherComp :type Primitive%20Component%20Object%20Reference) (OtherBodyIndex :type Integer) (bFromSweep :type Boolean) (SweepResult :type Hit%20Result%20Structure%20%28by%20ref%29))
  (bind (_color _intencity _description _colorname) (CallFunction|GetDTElem))
  (Utilities|FlowControl|Sequence
    (:then_0
      (Rendering|Components|Light|SetLightColor (Variables|Default|GetPointLight) _color true))
    (:then_1
      (Rendering|Components|Light|SetIntensity (Variables|Default|GetPointLight) _intencity))
    (:then_2
      (Development|PrintString (Utilities|String|Append (Utilities|String|ToString(Name) _colorname) ": " _description "        " "Count: " (Utilities|String|ToString(Integer) (Variables|Default|GetCrossCount)))))
    (:then_3
      (bind _result (Math|Integer|IncrementInt (Variables|Default|GetCrossCount))
        (:%20%20
          (Variables|Default|SetCrossCount _result))))))

(event EventBeginPlay
  (bind _outrownames (DataTable|GetDataTableRowNames "/Game/LooterShooter/Blueprint/DataBase/DT_Svetovor.DT_Svetovor"))
  (for (_array_element _array_index) _outrownames
    (bind _returnvalue (Utilities|GetDataTableRow "/Game/LooterShooter/Blueprint/DataBase/DT_Svetovor.DT_Svetovor" _array_element)
      (:then
        (Utilities|Array|AppendArray (Variables|Default|GetOut%20Row) (Utilities|Array|MakeArray _returnvalue))))))

(fn ConstructionScript)

(fn GetDTElem
  (bind _crosscount (Variables|Default|GetCrossCount))
  (bind _out_row (Variables|Default|GetOut%20Row))
  (bind _returnvalue (Math|Integer|%(Integer) _crosscount 3))
  (bind _output (Utilities|Array|Get(acopy) _out_row _returnvalue))
  (bind (_color _intencity _colorname _description) (Utilities|Struct|BreakS_SvetovorLights _output))
  (return _color _intencity _description _colorname))